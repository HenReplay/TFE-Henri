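; Enemy AI pawn that chases the player and ends the game by loading the death screen level on reaching them.
; PawnSensing sightings set a seeing flag, never cleared here, and trigger a follow event that runs AI MoveTo toward player zero.
; A successful move passes a CanAttack gate, re-armed on each follow call, then opens the level, hides the cursor and sets game-only input.
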(event OnSeePawn(PawnSensing)
  (params (Pawn :type Pawn%20Object%20Reference))
  (Variables|Default|SetisSeeingPlayer true)
  (CallFunction|FollowPlayer))

(event Custom|followPlayer
  (bind _returnvalue (Game|GetPlayerController 0))
  (Variables|Default|SetcanAttack true)
  (if (Variables|Default|GetisSeeingPlayer)
    (AI|AIMoveTo self "0, 0, 0" (Game|GetPlayerCharacter 0) 7e+01 false
      (:OnSuccess
        (if (Variables|Default|GetcanAttack)
          (Variables|Default|SetcanAttack false)
          (Game|OpenLevel(byName) "deathScreenMap")
          (Variables|/Script/Engine.PlayerController|SetbShowMouseCursor _returnvalue false)
          (Input|SetInputModeGameOnly _returnvalue false))))))

(event EventBeginPlay)

(event Collision|EventActorBeginOverlap
  (params (OtherActor :type Actor%20Object%20Reference)))

(event EventTick
  (params (DeltaSeconds :type Float%20%28single-precision%29)))

(fn ConstructionScript)